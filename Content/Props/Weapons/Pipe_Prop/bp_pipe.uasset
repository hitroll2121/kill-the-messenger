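; Pipe prop that serves as a hand-held melee weapon, attached through the first-person player controller when an interaction finishes.
; The RepNotify HasCollision toggles physics simulation and Pawn blocking, and is switched off on pickup.
; Left click fakes a swing with two timed relative rotations, then line-traces briefly forward from the holder's camera to apply damage, leaving persistent debug drawing.
; An override supplies the melee hand socket.
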(event Custom|hit
  (bind _returnvalue (Actor|GetAttachParentActor))
  (bind _returnvalue_2 (Actor|GetComponentbyClass _returnvalue "/Script/Engine.CameraComponent"))
  (bind _returnvalue_3 (Transformation|GetWorldLocation _returnvalue_2))
  (Transformation|SetActorRelativeRotation "-90.000000,0.000000,0.000000")
  (Utilities|FlowControl|Delay 0.2)
  (Transformation|SetActorRelativeRotation "-10.000000,0.000000,0.000000")
  (bind _outhit (Class|KismetSystemLibrary|LineTraceSinglebyProfile _returnvalue_3 (+ _returnvalue_3 (* (Math|Vector|GetForwardVector (Transformation|GetWorldRotation _returnvalue_2)) 1e+02)) "BlockAll" false (Utilities|Array|MakeArray (Actor|GetAttachParentActor)) "Persistent" true))
  (if (.bblockinghit _outhit)
    (Game|Damage|ApplyDamage (.hitactor _outhit) 1e+01 0 (Actor|GetAttachParentActor))))

(event EventBeginPlay
  (Variables|Default|SetHas%20collision true))

(event Collision|EventActorBeginOverlap
  (params (OtherActor :type Actor%20Object%20Reference)))

(event EventTick
  (params (DeltaSeconds :type Float%20%28single-precision%29)))

(event EventToggleCollison
  (params (Collsion :type Boolean))
  (Variables|Default|SetHas%20collision Collsion))

(event EventInteractLClick
  (CallFunction|Hit))

(event EventInteractFinish
  (params (actor :type Actor%20Object%20Reference) (playercontroller :type Actor%20Object%20Reference))
  (bind _asbp_first_person_player_controller (Utilities|Casting|CastToBP_FirstPersonPlayerController playercontroller))
  (Variables|Default|SetHas%20collision false)
  (Default|RunHandAnywhere _asbp_first_person_player_controller self "GripPoint" (Game|Player|GetPlayerPawn 0)))

(fn ConstructionScript)

(fn OnRepHasCollision
  (bind _has_collision (Variables|Default|GetHas%20collision))
  (bind _pipe (Variables|Default|GetPipe))
  (Physics|SetSimulatePhysics _pipe _has_collision)
  (if _has_collision
    (Collision|SetCollisionResponsetoChannel _pipe "ECC_Pawn" "ECR_Block")
    (else
      (Collision|SetCollisionResponsetoChannel _pipe "ECC_Pawn" "ECR_Ignore"))))

(fn CanInteract
  (params (actor :type Actor%20Object%20Reference))
  (return false))

(fn Interact
  (return 0.5))

(fn OverrideSocket
  (return false true "melee_weapon" "None"))